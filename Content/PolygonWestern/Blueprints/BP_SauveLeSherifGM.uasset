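; Game mode for SauveLeSherif that drives the match phase.
; On BeginPlay it steps through three phases separated by fixed delays, writing each to CurrentPhase on BP_SauveLeSherifGS through SetGamePhase.
; AssignRoles is an unfinished stub, not called here, that shuffles all BP_SauveLeSherifPS player states and casts the first without setting any role.
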(event EventBeginPlay
  (CallFunction|SetGamePhase "NewEnumerator0")
  (Utilities|FlowControl|Delay 5.0)
  (CallFunction|SetGamePhase "NewEnumerator1")
  (Utilities|FlowControl|Delay 5.0)
  (CallFunction|SetGamePhase "NewEnumerator2"))

(event EventTick
  (params (DeltaSeconds :type Float%20%28single-precision%29)))

(fn ConstructionScript)

(fn SetGamePhase
  (params (NewPhase :type E_GamePhase%20Enum :default "NewEnumerator0"))
  (bind _asbp_sauve_le_sherif_gs (Utilities|Casting|CastToBP_SauveLeSherifGS (Game|GetGameState)))
  (Variables|/Game/PolygonWestern/Blueprints/BP_SauveLeSherifGS.BP_SauveLeSherifGS_C|SetCurrentPhase _asbp_sauve_le_sherif_gs NewPhase))

(fn AssignRoles
  (bind _outactors (Actor|GetAllActorsOfClass "/Game/PolygonWestern/Blueprints/BP_SauveLeSherifPS.BP_SauveLeSherifPS_C"))
  (bind _output_get (Variables|Default|SetShuffledPlayers _outactors))
  (Utilities|Array|Shuffle _output_get)
  (Utilities|Casting|CastToBP_SauveLeSherifPS (Utilities|Array|Get(acopy) _output_get)))